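; Player actor for the Adam and Eve minigame, built to slide sideways and collect fruit.
; Tick makes swept moves along Y at a fixed per-frame step while an arrow flag is set.
; A cast chain scores and destroys ordinary fruit or prints game over for forbidden fruit.
; That chain and the flag setters are disconnected, and the Cube hit event is empty, so neither collection nor input works here.
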(event OnComponentHit(Cube)
  (params (HitComponent :type Primitive%20Component%20Object%20Reference) (OtherActor :type Actor%20Object%20Reference) (OtherComp :type Primitive%20Component%20Object%20Reference) (NormalImpulse :type Vector :default "0, 0, 0") (Hit :type Hit%20Result%20Structure%20%28by%20ref%29)))

(event EventBeginPlay)

(event Collision|EventActorBeginOverlap
  (params (OtherActor :type Actor%20Object%20Reference)))

(event EventTick
  (params (DeltaSeconds :type Float%20%28single-precision%29))
  (bind _returnvalue (Transformation|GetActorLocation))
  (bind _returnvalue_2 (Transformation|GetActorLocation))
  (if (Variables|Default|GetLeftArrowDown)
    (Transformation|SetActorLocation (Math|Vector|MakeVector (.x _returnvalue_2) (- (.y _returnvalue_2) 5.0) (.z _returnvalue_2)) true false)
    (elif (Variables|Default|GetRightArrowDown)
      (Transformation|SetActorLocation (Math|Vector|MakeVector (.x _returnvalue) (+ (.y _returnvalue) 5.0) (.z _returnvalue)) true false))))

(fn ConstructionScript)

(fn AddScore
  (params (score :type Integer))
  (Variables|Default|SetScore (+ (Variables|Default|GetScore) score)))