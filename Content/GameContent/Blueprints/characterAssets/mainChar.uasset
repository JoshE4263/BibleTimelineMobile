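; Main character Blueprint that holds an inventory and moves sideways along world Y from screen-edge touches.
; PutinInventory appends an item struct and refreshes the main HUD.
; TestMouseScreenPos nudges the actor without sweep while the touch is near either viewport edge, within Y limits, and sets IsMoving.
; Helpers latch left-mouse state and return the current attachment; older AddMovementInput logic is left unconnected.
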(event EventBeginPlay)

(event Collision|EventActorBeginOverlap
  (params (OtherActor :type Actor%20Object%20Reference)))

(event EventPutinInventory
  (params (InventoryStruct :type Inventory%20Struct%20Structure))
  ;[1 1 1] Put in Inventory - Verified and working - 8/15/18
  (Utilities|Array|Add (Variables|Default|GetInventory) InventoryStruct)
  (Default|RefreshInventory (Variables|Default|GetMainUIHUD)))

(fn ConstructionScript)

(fn SetMouseButtonDown
  (params (MouseDown :type Boolean))
  (if MouseDown
    (Utilities|FlowControl|DoOnce false :!label _label
      (:Completed
        (Variables|Default|SetLMB_Down true)))
    (else
      (Variables|Default|SetLMB_Down false)
      (goto _label Reset))))

(fn TestMouseScreenPos
  (params (touchLocation :type Vector))
  (if (> (.x touchLocation) (- (.x (Viewport|GetViewportSize)) 2e+02))
    (if (< (.y (Transformation|GetActorLocation)) (Variables|Default|GetMaxYVal))
      (Transformation|SetActorLocation (+ (Transformation|GetActorLocation) "0.000000,10.000000, 0") false false)
      (Variables|Default|SetisMoving true))
    (elif (< (.x touchLocation) 2e+02)
      (if (> (.y (Transformation|GetActorLocation)) (Variables|Default|GetMinYVal))
        (Transformation|SetActorLocation (+ (Transformation|GetActorLocation) "0.000000,-10.000000, 0") false false)
        (Variables|Default|SetisMoving true))
      (else
        (Variables|Default|SetisMoving false)))))

(fn GetActualAttached
  (return (Variables|Default|GetcurrentAttached)))